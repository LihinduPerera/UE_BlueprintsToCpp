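; BP_Door is a door actor that swings itself open at BeginPlay, then calls CloseDoor five seconds later.
; OpenDoor and CloseDoor set a positive or negative yaw step and raise a flag that enables rotation in Tick.
; Tick adds that fixed step each frame, independent of delta time, until world yaw passes +90 when opening or -90 when closing, then clears the flag.
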(event `self.ReceiveBeginPlay`
  (`self.OpenDoor`)
  (`KismetSystemLibrary.Delay` 5.0)
  (`self.CloseDoor`))

(event `self.ReceiveTick`
  (params (DeltaSeconds :type "Float (single-precision)"))
  (bind (_returnvalue_roll _returnvalue_pitch _returnvalue_yaw) (`KismetMathLibrary.BreakRotator` (`self.K2_GetActorRotation`)))
  (bind (_returnvalue_roll_2 _returnvalue_pitch_2 _returnvalue_yaw_2) (`KismetMathLibrary.BreakRotator` (`self.K2_GetActorRotation`)))
  (bind (_returnvalue_roll_3 _returnvalue_pitch_3 _returnvalue_yaw_3) (`KismetMathLibrary.BreakRotator` (`self.K2_GetActorRotation`)))
  (if (`self.ShouldOpenOrClose`)
    (`self.K2_SetActorRotation` (`KismetMathLibrary.MakeRotator` _returnvalue_roll _returnvalue_pitch (+ _returnvalue_yaw (`self.Yaw Increment`))))
    (if (or (and (> (`self.Yaw Increment`) 0.0) (>= _returnvalue_yaw_2 90.0)) (and (< (`self.Yaw Increment`) 0.0) (<= _returnvalue_yaw_3 -90.0)))
      (set `self.ShouldOpenOrClose` false))))

(event `OpenDoor`
  (set `self.Yaw Increment` 2.0)
  (set `self.ShouldOpenOrClose` true))

(event `CloseDoor`
  (set `self.Yaw Increment` -2.0)
  (set `self.ShouldOpenOrClose` true))

(fn `UserConstructionScript`)